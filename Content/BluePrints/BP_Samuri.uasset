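; BP_Samuri is a samurai sprite Blueprint that slides its PaperSprite into place when play begins.
; BeginPlay caches the sprite's relative location as its resting position, then calls the SlideIn event.
; SlideIn plays the SlideInAni timeline from the start at double rate, using its Alpha to lerp the sprite from SlideStartPos to that cached position.
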(event Custom|SlideIn
  (Components|Timeline|SetPlayRate (Variables|Default|GetSlideInAni) 2.0)
  (bind _alpha (Timeline|SlideInAni PlayFromStart)
    (:Update
      (Transformation|SetRelativeLocation (Variables|Default|GetPaperSprite) (Math|Vector|Lerp(Vector) (Variables|Default|GetSlideStartPos) (Variables|Default|GetSpriteDefaultPos) _alpha) false false))))

(event EventBeginPlay
  (Variables|Default|SetSpriteDefaultPos (Variables|/Script/Engine.SceneComponent|GetRelativeLocation (Variables|Default|GetPaperSprite)))
  (CallFunction|Slidein))

(event Collision|EventActorBeginOverlap
  (params (OtherActor :type Actor%20Object%20Reference)))

(event EventTick
  (params (DeltaSeconds :type Float%20%28single-precision%29)))

(fn ConstructionScript)